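; Companion character that guides the player toward unvisited landmarks and performs echolocation, with sound cues loaded from a data table.
; It feeds the next landmark (lowest order number, nearest on ties) to its AI Blackboard, updating on each visit.
; Echolocation sphere-traces for I_EchoLocation actors, then a timeline reveals hits by distance like an expanding wave, and Tick expires highlights.
; It can also turn toward the player and interpolate mesh elevation.
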(event Custom|EchoLocate
  (bind _returnvalue (Transformation|GetActorLocation))
  (bind _returnvalue_2 (Transformation|GetActorLocation))
  ;[1 1 1] EchoLocation
  (Utilities|Map|Clear (Variables|Default|GetEchoHits))
  (Audio|PlaySoundatLocation (.sound (Variables|Default|GetEchoSendSound)) _returnvalue_2 "0, 0, 0" 0.1 1.0 0.0 0 0 self 0)
  (Niagara|SpawnSystematLocation "/Game/Blueprints/Companion/FX/NS_EchoLocation.NS_EchoLocation" _returnvalue_2)
  ;;[1 1 1] Collect all relevant hits
  (bind _outhits (Collision|MultiSphereTraceByChannel _returnvalue (+ _returnvalue "0.000000,0.000000,1.000000") (Variables|Default|GetEchoDistance) "TraceTypeQuery1" false 0 "None"))
  (for _array_element _outhits
    (if (Utilities|DoesObjectImplementInterface (.HitActor (Collision|BreakHitResult _array_element)) "/Game/Blueprints/Companion/I_EchoLocation.I_EchoLocation_C")
      (Utilities|Map|Add (Variables|Default|GetEchoHits) (Transformation|GetDistanceTo (.HitActor (Collision|BreakHitResult _array_element)) self) (.HitActor (Collision|BreakHitResult _array_element)))))
  (bind _keys (Utilities|Map|Keys (Variables|Default|GetEchoHits)))
  (bind _output_get (Variables|Default|SetRemainingHits _keys))
  (if (> (Utilities|Array|Length _output_get) 0)
    (bind _distancescale (Timeline|EchoLocateScan PlayFromStart)
      (:Update
        (CallFunction|CheckEchoHits _distancescale (Variables|Default|GetRemainingHits))))))

(event Custom|SayHi
  ;[1 1 1] Ping player
  (Audio|PlaySoundatLocation (.sound (Variables|Default|GetHereSound)) (Transformation|GetActorLocation) "0, 0, 0" 0.1 1.0 0.0 0 0 self 0))

(event Custom|StartInterpElevation
  (params (ElevationTarget :type Float%20%28double-precision%29) (PlayRate :type Float%20%28single-precision%29))
  (bind _mesh (Variables|Character|GetMesh))
  (Components|Timeline|SetPlayRate (Variables|Default|GetInterpElevation) PlayRate)
  (Variables|Default|SetElevationTarget ElevationTarget)
  (Variables|Default|SetStartElevation (.z (Variables|/Script/Engine.SceneComponent|GetRelativeLocation _mesh)))
  (bind _interpheight (Timeline|InterpElevation PlayFromStart)
    (:Update
      (Transformation|SetRelativeLocation _mesh (Math|Vector|MakeVector 0.0 0.0 (Math|Float|MapRangeClamped _interpheight 0.0 1.0 (Variables|Default|GetStartElevation) (Variables|Default|GetElevationTarget))) false false))))

(event Custom|SetOrientToPlayer
  (params (bOrientToPlayer :type Boolean))
  (bind _output_get (Variables|Default|SetbOrientToPlayer bOrientToPlayer))
  (Variables|/Script/Engine.CharacterMovementComponent|SetbOrientRotationToMovement (Variables|Character|GetCharacterMovement) (not _output_get)))

(event EventBeginPlay
  ;[1 1 1] Begin Play
  (CallFunction|LoadSoundCues)
  (bind _asbp_third_person_character (Utilities|Casting|CastToBP_ThirdPersonCharacter (Game|GetPlayerCharacter 0) :!label _label)
    (:then
      (Variables|Default|SetLuna _asbp_third_person_character)
      (EventDispatchers|AssignOnEchoLocatePressed _asbp_third_person_character (EventDispatchers|CreateEvent :!event Custom|EchoLocate))
      (bind _outactors (Actor|GetAllActorsOfClass "/Game/Blueprints/Landmarks/Landmark_Master.Landmark_Master_C"))
      (for _array_element _outactors
        (if (not (Variables|/Game/Blueprints/Landmarks/Landmark_Master.Landmark_Master_C|GetLandmarkWasVisited _array_element))
          (Utilities|Array|Add (Variables|Default|GetLandmarks) _array_element)
          (EventDispatchers|AssignOnLandmarkVisited _array_element (EventDispatchers|CreateEvent :!event OnLandmarkVisited))))
      (CallFunction|SetNextLandmark))
    (:CastFailed
      (Utilities|FlowControl|Delay 0.2)
      (goto _label))))

(event EventTick
  (params (DeltaSeconds :type Float%20%28single-precision%29))
  ;[1 1 1] Tick
  (CallFunction|OrienttoPlayer DeltaSeconds)
  (Variables|Default|SetSpeed (Math|Vector|VectorLength (Variables|/Script/Engine.MovementComponent|GetVelocity (Variables|Character|GetCharacterMovement))))
  (CallFunction|UnhighlightActors))

(fn ConstructionScript)

(fn LoadSoundCues
  (Utilities|FlowControl|Sequence
    (:then_0
      (bind _returnvalue (Utilities|GetDataTableRow "/Game/Blueprints/Companion/DT_CompanionSounds.DT_CompanionSounds" "Warn")
        (:then
          (Variables|Default|SetWarnSound _returnvalue))))
    (:then_1
      (bind _returnvalue_2 (Utilities|GetDataTableRow "/Game/Blueprints/Companion/DT_CompanionSounds.DT_CompanionSounds" "Here")
        (:then
          (Variables|Default|SetHereSound _returnvalue_2))))
    (:then_2
      (bind _returnvalue_3 (Utilities|GetDataTableRow "/Game/Blueprints/Companion/DT_CompanionSounds.DT_CompanionSounds" "Echo")
        (:then
          (Variables|Default|SetEchoSendSound _returnvalue_3))))
    (:then_3
      (bind _returnvalue_4 (Utilities|GetDataTableRow "/Game/Blueprints/Companion/DT_CompanionSounds.DT_CompanionSounds" "EchoHit")
        (:then
          (Variables|Default|SetEchoHitSound _returnvalue_4))))))

(fn CheckEchoHits
  (params (Scale :type Float%20%28double-precision%29) (Array :type Array%20of%20Floats%20%28double-precision%29))
  (bind _output_get (LocalVariables|SetKeys Array))
  (for _array_element _output_get
    (if (<= _array_element (* Scale (Variables|Default|GetEchoDistance)))
      (CallFunction|AddHighlightActor (.Value (Utilities|Map|Find (Variables|Default|GetEchoHits) _array_element)))
      (Class|IEchoLocation|EchoHit(Message) (.Value (Utilities|Map|Find (Variables|Default|GetEchoHits) _array_element)))
      (Utilities|Array|RemoveItem (Variables|Default|GetRemainingHits) _array_element))))

(fn UnhighlightActors
  (bind _highlightedactors (Variables|Default|GetHighlightedActors))
  (bind _output (Utilities|Array|Get(acopy) _highlightedactors))
  (if (> (Utilities|Array|Length (Variables|Default|GetHighlightedActors)) 0) :!label _label
    (if (< (+ (.float _output) 5.0) (Actor|GetGameTimeSinceCreation (Game|GetGameState)))
      (Class|IEchoLocation|EchoEnd(Message) (.actor _output))
      (Utilities|Array|RemoveIndex (Variables|Default|GetHighlightedActors))
      (goto _label))))

(fn AddHighlightActor
  (params (Actor :type Actor%20Object%20Reference))
  (for (_array_element _array_index) (Variables|Default|GetHighlightedActors)
    (if (== (.Actor (Utilities|Struct|BreakS_ActorFloat _array_element)) Actor)
      (Utilities|Array|RemoveIndex (Variables|Default|GetHighlightedActors) _array_index)
      (Utilities|Array|Add (Variables|Default|GetHighlightedActors) (Utilities|Struct|MakeS_ActorFloat Actor (Actor|GetGameTimeSinceCreation (Game|GetGameState))))
      (return)))
  (Utilities|Array|Add (Variables|Default|GetHighlightedActors) (Utilities|Struct|MakeS_ActorFloat Actor (Actor|GetGameTimeSinceCreation (Game|GetGameState))))
  (return))

(fn OnLandmarkVisited
  (params (Landmark :type Landmark%20Master%20Object%20Reference))
  (Utilities|Array|RemoveItem (Variables|Default|GetLandmarks) Landmark)
  (CallFunction|SetNextLandmark))

(fn GetNextLandmark
  (for _array_element (Variables|Default|GetLandmarks)
    (Utilities|IsValid (LocalVariables|GetNextLandmark)
      (:Is%20Valid
        (if (> (Variables|/Game/Blueprints/Landmarks/Landmark_Master.Landmark_Master_C|GetLandmarkOrderNumber (LocalVariables|GetNextLandmark)) (Variables|/Game/Blueprints/Landmarks/Landmark_Master.Landmark_Master_C|GetLandmarkOrderNumber _array_element))
          (LocalVariables|SetNextLandmark _array_element :!label _label)
          (elif (== (Variables|/Game/Blueprints/Landmarks/Landmark_Master.Landmark_Master_C|GetLandmarkOrderNumber (LocalVariables|GetNextLandmark)) (Variables|/Game/Blueprints/Landmarks/Landmark_Master.Landmark_Master_C|GetLandmarkOrderNumber _array_element))
            (if (> (Class|Actor|GetSquaredHorizontalDistanceto (LocalVariables|GetNextLandmark)) (Class|Actor|GetSquaredHorizontalDistanceto _array_element))
              (goto _label)))))
      (:Is%20Not%20Valid
        (goto _label))))
  (return (LocalVariables|GetNextLandmark)))

(fn OrienttoPlayer
  (params (DeltaTime :type Float%20%28double-precision%29))
  (if (Variables|Default|GetbOrientToPlayer)
    (Transformation|SetActorRotation (Math|Rotator|MakeRotator 0.0 0.0 (.yaw (Math|Interpolation|RInterpTo (Transformation|GetActorRotation) (Math|Rotator|FindLookatRotation (Transformation|GetActorLocation) (Transformation|GetActorLocation (Variables|Default|GetLuna))) DeltaTime 2.0))))))

(fn SetNextLandmark
  (AI|Components|Blackboard|SetValueasObject (AI|GetBlackboard 0) (Utilities|Name|MakeLiteralName "NextLandmark") (CallFunction|GetNextLandmark)))