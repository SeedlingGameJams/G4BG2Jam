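; Health component for its owning actor that tracks current and maximum health.
; On BeginPlay it binds to the owner's OnTakeAnyDamage and fills health from a default value.
; Damage and healing clamp health between zero and max, broadcasting damage, death, heal and health-changed events.
; Changing max health rescales current health to keep the same percentage and notifies listeners.
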(event Custom|Heal
  (params (Amount :type Float%20%28double-precision%29))
  ;[1 1 1] Heal
  (if (!= (Variables|Default|GetMaxHealth) (Variables|Default|GetHealth))
    (Utilities|FlowControl|Sequence
      (:then_0
        (if (> (+ Amount (Variables|Default|GetHealth)) (Variables|Default|GetMaxHealth))
          (Variables|Default|SetHealth (Variables|Default|GetMaxHealth))
          (else
            (Variables|Default|SetHealth (+ Amount (Variables|Default|GetHealth))))))
      (:then_1
        (Default|CallOnHeal Amount)
        (Default|CallOnHealthChanged (Variables|Default|GetHealth))))))

(event Custom|OnTakeAnyDamage_Event
  (params (DamagedActor :type Actor%20Object%20Reference) (Damage :type Float%20%28single-precision%29) (DamageType :type Damage%20Type%20Object%20Reference) (InstigatedBy :type Controller%20Object%20Reference) (DamageCauser :type Actor%20Object%20Reference))
  ;[1 1 1] Apply damage to health component
  (if (CallFunction|IsAlive)
    (if (> (- (Variables|Default|GetHealth) Damage) 0.0)
      (bind _output_get (Variables|Default|SetHealth (- (Variables|Default|GetHealth) Damage)))
      (Default|CallOnDamaged)
      (Default|CallOnHealthChanged _output_get)
      (else
        (Variables|Default|SetHealth 0.0)
        (Default|CallOnDeath)
        (Default|CallOnHealthChanged 0.0)))))

(event EventBeginPlay
  ;[1 1 1] Assign On Damage taken from owner
  (EventDispatchers|AssignOnTakeAnyDamage (Components|GetOwner) (EventDispatchers|CreateEvent :!event Custom|OnTakeAnyDamage_Event))
  (bind _output_get (Variables|Default|SetMaxHealth (Variables|Default|GetDefaultHealth)))
  (Variables|Default|SetHealth _output_get))

(fn IsAlive
  (return (> (Variables|Default|GetHealth) 0.0)))

(fn GetHealth
  (return (Variables|Default|GetHealth)))

(fn ChangeMaxHealth
  (params (NewMaxHealth :type Float%20%28double-precision%29))
  (LocalVariables|SetHealthPercent (/ (Variables|Default|GetHealth) (Variables|Default|GetMaxHealth)))
  (bind _output_get (Variables|Default|SetMaxHealth NewMaxHealth))
  (Variables|Default|SetHealth (* _output_get (LocalVariables|GetHealthPercent)))
  (Default|CallOnMaxHealthChanged (Variables|Default|GetMaxHealth))
  (Default|CallOnHealthChanged (Variables|Default|GetHealth)))

(fn GetMaxHealth
  (return (Variables|Default|GetMaxHealth)))