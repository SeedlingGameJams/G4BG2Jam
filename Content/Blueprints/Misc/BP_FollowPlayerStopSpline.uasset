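; BP_FollowPlayerStopSpline is a spline actor that supplies the closest point on its path to a given actor, apparently for follow-player stop logic.
; Its construction script lays a spline mesh component along each segment between neighboring points, matching locations and tangents, and hides each one.
; FindActorLocation returns the X, Y and Z of the world-space spline location nearest the passed actor.
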(fn ConstructionScript
  (for _index (range 0 (- (Spline|GetNumberOfSplinePoints (Variables|Default|GetSpline)) 2))
    (bind _returnvalue (AddComponent|AddSplineMeshComponent false))
    (Transformation|AttachComponentToComponent _returnvalue (Variables|Default|GetSpline) "None" "KeepRelative" "KeepRelative" "KeepRelative" true)
    (SplineMesh|SetStartandEnd _returnvalue (.Location (Spline|GetLocationandTangentatSplinePoint (Variables|Default|GetSpline) _index "Local")) (.Tangent (Spline|GetLocationandTangentatSplinePoint (Variables|Default|GetSpline) _index "Local")) (.Location (Spline|GetLocationandTangentatSplinePoint (Variables|Default|GetSpline) (+ _index 1) "Local")) (.Tangent (Spline|GetLocationandTangentatSplinePoint (Variables|Default|GetSpline) (+ _index 1) "Local")) true :!class /Script/Engine.SplineMeshComponent)
    (Rendering|SetVisibility _returnvalue false false)))

(fn FindActorLocation
  (params (Actor :type Actor%20Object%20Reference))
  (bind _returnvalue (Transformation|GetActorLocation Actor))
  (bind _spline (Variables|Default|GetSpline))
  (bind _returnvalue_2 (Spline|FindLocationClosesttoWorldLocation _spline _returnvalue "World"))
  (return (.x _returnvalue_2) (.y _returnvalue_2) (.z _returnvalue_2)))