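; Spline-based blocker actor that slides blocking components along a spline to track the player (TPC_Luna) and a companion, marked OLD in its name.
; Looping timers drive the updates, with the player's started on BeginPlay and the companion's by BeginCompanionBlocking.
; FindActorLocation supplies the closest spline point for each blocker, and PlayerBlocker also takes the spline's yaw.
; Despite its name, MoveAudio moves PlayerBlocker; the companion reference is not assigned in these graphs.
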(event Custom|MoveAudio
  (bind _playerblocker (Variables|Default|GetPlayerBlocker))
  (bind _as_tpc_luna (Variables|Default|GetAs%20TPC%20Luna))
  (bind (_returnvalue_x _returnvalue_y _returnvalue) (CallFunction|FindActorLocation _as_tpc_luna))
  (Transformation|SetWorldLocation _playerblocker (Math|Vector|MakeVector _returnvalue_x _returnvalue_y _returnvalue) false false)
  (Transformation|SetRelativeRotation _playerblocker (Math|Rotator|MakeRotator 0.0 0.0 (.Yaw (Math|Rotator|BreakRotator (Class|SplineComponent|FindRotationClosesttoWorldLocation (Variables|Default|GetSpline) (Transformation|GetActorLocation _as_tpc_luna) "Local")))) false false))

(event Custom|CompanionBlockerLooper
  (bind (_returnvalue_x _returnvalue_y _returnvalue) (CallFunction|FindActorLocation (Variables|Default|GetAsCompanion)))
  (Transformation|SetWorldLocation (Variables|Default|GetCompanionBlocker) (Math|Vector|MakeVector _returnvalue_x _returnvalue_y _returnvalue) false false))

(event Custom|BeginCompanionBlocking
  (if (not (Utilities|Time|IsTimerActivebyHandle (Variables|Default|GetTmrCompanionBlocker)))
    (bind _returnvalue (Utilities|Time|SetTimerbyEvent (EventDispatchers|CreateEvent :!event Custom|CompanionBlockerLooper) 0.05 true))
    (Variables|Default|SetTmrCompanionBlocker _returnvalue)))

(event EventBeginPlay
  (Utilities|FlowControl|DelayUntilNextTick)
  (bind _astpc_luna (Utilities|Casting|CastToTPC_Luna (Game|GetPlayerCharacter 0)))
  (Variables|Default|SetAs%20TPC%20Luna _astpc_luna)
  (if (not (Class|KismetSystemLibrary|TimerExistsHandle (Variables|Default|GetTmrUpdateTime)))
    (bind _returnvalue (Utilities|Time|SetTimerbyEvent (EventDispatchers|CreateEvent :!event Custom|MoveAudio) 0.05 true))
    (Variables|Default|SetTmrUpdateTime _returnvalue)))

(fn ConstructionScript)

(fn FindActorLocation
  (params (Actor :type Actor%20Object%20Reference))
  (bind _returnvalue (Transformation|GetActorLocation Actor))
  (bind _spline (Variables|Default|GetSpline))
  (bind _returnvalue_2 (Spline|FindLocationClosesttoWorldLocation _spline _returnvalue "World"))
  (return (.x _returnvalue_2) (.y _returnvalue_2) (.z _returnvalue_2)))