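; Base interactible Blueprint for world objects the player can interact with.
; Its interaction event forwards to an OnPlayerInteractsWithObject dispatcher.
; A collision component's overlap events drive a notification marker, with both begin and end overlap setting it and its children visible, so nothing here hides it again.
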(event OnComponentBeginOverlap(Collision)
  (params (OverlappedComponent :type Primitive%20Component%20Object%20Reference) (OtherActor :type Actor%20Object%20Reference) (OtherComp :type Primitive%20Component%20Object%20Reference) (OtherBodyIndex :type Integer) (bFromSweep :type Boolean) (SweepResult :type Hit%20Result%20Structure%20%28by%20ref%29))
  (bind _notification_marker (Variables|Default|GetNotification%20Marker))
  (if (Utilities|IsValid _notification_marker)
    (Rendering|SetVisibility (Variables|/Game/Blueprints/Interactible/InteractionNotification.InteractionNotification_C|GetDefaultSceneRoot _notification_marker) true true)))

(event OnComponentEndOverlap(Collision)
  (params (OverlappedComponent :type Primitive%20Component%20Object%20Reference) (OtherActor :type Actor%20Object%20Reference) (OtherComp :type Primitive%20Component%20Object%20Reference) (OtherBodyIndex :type Integer))
  (bind _notification_marker (Variables|Default|GetNotification%20Marker))
  (if (Utilities|IsValid _notification_marker)
    (Rendering|SetVisibility (Variables|/Game/Blueprints/Interactible/InteractionNotification.InteractionNotification_C|GetDefaultSceneRoot _notification_marker) true true)))

(event EventInteractionEvent
  (Default|CallOnPlayerInteractswithObject))

(fn ConstructionScript)