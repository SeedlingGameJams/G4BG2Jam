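; Interactible grave piece that Luna picks up, with a check for whether it is the last one in the level.
; On interaction it plays a pickup animation on the player's mesh, then restores the Animation Blueprint after a fixed delay.
; In parallel it counts all grave part actors, destroying itself after the same delay if others remain.
; The last piece only prints a message and is not destroyed.
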(event EventInteractionEvent
  (Utilities|FlowControl|Sequence
    (:then_0
      (bind _astpc_luna (Utilities|Casting|CastToTPC_Luna (Game|Player|GetPlayerPawn 0)))
      (Components|Animation|PlayAnimation (Variables|/Script/Engine.Character|GetMesh _astpc_luna) "/Game/ArtAssets/PlayerCharacter/Animations/AN_PickUp.AN_PickUp" false)
      (Utilities|FlowControl|Delay 1.4) ; Set to animation duration
      (Components|Animation|SetAnimationMode (Variables|/Script/Engine.Character|GetMesh _astpc_luna) "AnimationBlueprint"))
    (:then_1
      (bind _outactors (Actor|GetAllActorsOfClass "Interactible_GraveParts_C"))
      (for _array_element _outactors
        (Variables|Default|SetCount (+ (Variables|Default|GetCount) 1)))
      (if (<= (Variables|Default|GetCount) 1)
        (Development|PrintText "THIS IS THE LAST PIECE" true true "(R=1.000000,G=0.005617,B=0.000000,A=1.000000)")
        (else
          (Utilities|FlowControl|Delay 1.4) ; Set to animation duration
          (Actor|DestroyActor))))))

(fn ConstructionScript
  (|CallParentFunction))