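; Pickup stone interactible, a child Blueprint that plays the SEQ_BuryCompanion level sequence and removes itself when the player interacts with it.
; On pickup it loops over all Interactible_Stone_Child actors, incrementing InteractablesLeft for each.
; The count check sits inside the loop body, so the sequence fires whenever the running count equals 1, rather than testing the final total, and every branch destroys the stone.
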(event Custom|On%20Pick%20UP
  (bind _outactors (Actor|GetAllActorsOfClass "Interactible_Stone_Child_C"))
  (for _array_element _outactors
    (bind _output_get (Variables|Default|SetInteractablesLeft (+ (stale _output_get) 1)))
    (if (== _output_get 1)
      (bind _outactor (Sequencer|Player|CreateLevelSequencePlayer "/Game/Sequences/SEQ_BuryCompanion.SEQ_BuryCompanion"))
      (Sequencer|Player|Play (Variables|/Script/LevelSequence.LevelSequenceActor|GetSequencePlayer _outactor) :!class /Script/MovieScene.MovieSceneSequencePlayer)
      (Actor|DestroyActor)
      (else
        (Actor|DestroyActor)))))

(event EventBeginPlay
  (EventDispatchers|BindEventtoOnPlayerInteractswithObject (delegate Custom|On%20Pick%20UP)))

(event Collision|EventActorBeginOverlap
  (params (OtherActor :type Actor%20Object%20Reference)))

(event EventTick
  (params (DeltaSeconds :type Float%20%28single-precision%29)))

(fn ConstructionScript
  (|CallParentFunction))