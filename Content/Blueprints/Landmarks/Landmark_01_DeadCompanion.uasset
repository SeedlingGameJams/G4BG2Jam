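; Landmark Blueprint for the dead companion, which scatters grave part interactibles around itself when the landmark finishes.
; On BeginPlay it binds to the parent's landmark-reached dispatcher and destroys its leading spline once reached.
; On finish it reveals the landmark mesh and spawns several Interactible_GraveParts at offset random navigable points nearby, adjusting for collision but always spawning.
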(event Custom|OnLandmarkReached_Event
  (Actor|DestroyActor (Variables|Default|GetLeadingSpline)))

(event EventLandmarkFinished
  (|CallParentFunction)
  (Rendering|SetVisibility (Variables|Default|GetLandmarkMesh) true false)
  (for _index (range 0 2)
    (bind _randomlocation (Class|NavigationSystemV1|GetRandomLocationinNavigableRadius (Transformation|GetActorLocation) 7.5e+02 0 0))
    (Game|SpawnActorfromClass "/Game/Blueprints/Interactible/Interactible_GraveParts.Interactible_GraveParts_C" (Math|Transform|MakeTransform (+ _randomlocation "100.000000,100.000000,0.000000") "0, 0, 0" "1.000000,1.000000,1.000000") "AdjustIfPossibleButAlwaysSpawn" 0 0)))

(event EventBeginPlay
  (|CallParentFunction)
  (EventDispatchers|AssignOnLandmarkReached (delegate Custom|OnLandmarkReached_Event)))

(fn ConstructionScript)