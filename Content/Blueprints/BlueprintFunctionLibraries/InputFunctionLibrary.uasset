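; Blueprint function library that turns Enhanced Input actions into display names of their bound keyboard keys.
; Both functions scan an input mapping context's mappings and keep only keyboard keys, with optional long names.
; One returns the first match for an action; the other collects all matches whose player-mappable display category equals a given key group.
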(fn GetInputActionKey
  (params (InputAction :type Input%20Action%20Object%20Reference) (bLongDisplayName :type Boolean))
  (bind _array_element (Utilities|Array|ForEachLoopwithBreak (Variables|/Script/EnhancedInput.InputMappingContext|GetMappings (LocalVariables|GetInputContext)))
    (:LoopBody
      (if (== InputAction (.Action (Utilities|Struct|BreakEnhancedActionKeyMapping _array_element)))
        (if (Class|KismetInputLibrary|KeyIsKeyboardKey (.Key (Utilities|Struct|BreakEnhancedActionKeyMapping _array_element)))
          (return (Class|KismetInputLibrary|KeyGetDisplayName (.Key (Utilities|Struct|BreakEnhancedActionKeyMapping _array_element)) bLongDisplayName)))))))

(fn GetInputActionKeyGroup
  (params (InputAction :type Input%20Action%20Object%20Reference) (KeyGroup :type Text) (bLongDisplayName :type Boolean))
  (for _array_element (Variables|/Script/EnhancedInput.InputMappingContext|GetMappings (LocalVariables|GetInputContext))
    (if (Math|Boolean|ANDBoolean (== InputAction (.Action (Utilities|Struct|BreakEnhancedActionKeyMapping _array_element))) (Utilities|Enum|Equal(Enum) KeyGroup (.displaycategory (.PlayerMappableOptions (Utilities|Struct|BreakEnhancedActionKeyMapping _array_element)))) (Class|KismetInputLibrary|KeyIsKeyboardKey (.Key (Utilities|Struct|BreakEnhancedActionKeyMapping _array_element))))
      (if (Class|KismetInputLibrary|KeyIsKeyboardKey (.Key (Utilities|Struct|BreakEnhancedActionKeyMapping _array_element)))
        (Utilities|Array|Add (LocalVariables|GetReturnKeys) (Class|KismetInputLibrary|KeyGetDisplayName (.Key (Utilities|Struct|BreakEnhancedActionKeyMapping _array_element)) bLongDisplayName)))))
  (return (LocalVariables|GetReturnKeys)))