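; Base roaming NPC that wanders around the spot where it stands one second after BeginPlay and emits periodic sounds.
; AIMoveTo targets a random reachable point near that origin plus a positive X/Y offset, while a randomized timer started alongside each move request picks the next destination.
; A separate randomized timer loop replays the attached sound, starting at BeginPlay.
; Tick stores the movement speed.
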(event Custom|Random%20roam
  (AI|AIMoveTo self (+ (.RandomLocation (AI|Navigation|GetRandomReachablePointinRadius (Variables|Default|GetOrigin%20Point) (Variables|Default|GetRandom%20Radius) 0 0)) (Math|Vector|MakeVector (Math|Random|RandomFloatinRange 5e+02 1e+03) (Math|Random|RandomFloatinRange 5e+02 1e+03) 0.0)) 0 5.0 false
    (:then
      (if (not (Utilities|Time|IsTimerActivebyHandle (Variables|Default|GettmrDelay)))
        (bind _returnvalue (Utilities|Time|SetTimerbyEvent (delegate Custom|EndDelay) (Math|Random|RandomFloatinRange 3.0 1e+01)))
        (Variables|Default|SettmrDelay _returnvalue)))))

(event Custom|EndDelay
  (Utilities|Time|ClearandInvalidateTimerbyHandle (Variables|Default|GettmrDelay))
  (CallFunction|RandomRoam))

(event Custom|BeginMovement
  (Variables|Default|SetOrigin%20Point (Transformation|GetWorldLocation (Variables|Default|GetCapsuleComponent)))
  (CallFunction|RandomRoam))

(event Custom|DelayCall
  (Utilities|Time|ClearandInvalidateTimerbyHandle (Variables|Default|GettmrSoundCall))
  (CallFunction|PlaySoundAgain))

(event Custom|PlaySoundAgain
  (Audio|SpawnSoundAttached (Variables|Default|GetSoundToPlay) (Variables|Character|GetMesh) "None" "0, 0, 0" "0, 0, 0" "KeepRelativeOffset" false 1.0 1.0 0.0 0 0)
  (if (not (Utilities|Time|IsTimerActivebyHandle (Variables|Default|GettmrSoundCall)))
    (bind _returnvalue (Utilities|Time|SetTimerbyEvent (delegate Custom|DelayCall) (Math|Random|RandomFloatinRange 2.0 15.0)))
    (Variables|Default|SettmrSoundCall _returnvalue)))

(event EventBeginPlay
  ;[1 1 1] Allow spawn time
  (Utilities|Time|SetTimerbyEvent (delegate Custom|BeginMovement) 1.0)
  (Audio|SpawnSoundAttached (Variables|Default|GetSoundToPlay) (Variables|Character|GetMesh) "None" "0, 0, 0" "0, 0, 0" "KeepRelativeOffset" false 1.0 1.0 0.0 0 0)
  (if (not (Utilities|Time|IsTimerActivebyHandle (Variables|Default|GettmrSoundCall)))
    (bind _returnvalue (Utilities|Time|SetTimerbyEvent (delegate Custom|DelayCall) (Math|Random|RandomFloatinRange 2.0 15.0)))
    (Variables|Default|SettmrSoundCall _returnvalue)))

(event EventTick
  (params (DeltaSeconds :type Float%20%28single-precision%29))
  (Variables|Default|SetSpeed_0 (Math|Vector|VectorLength (Variables|/Script/Engine.MovementComponent|GetVelocity (Variables|Character|GetCharacterMovement)))))

(fn ConstructionScript)