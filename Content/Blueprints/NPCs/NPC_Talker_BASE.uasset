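; Base NPC dialogue actor that plays lines from a data table through the HUD's dialogue textbox.
; Collision overlap or remote events cache the textbox, auto-starting dialogue if TouchActivated; leaving hides it.
; Each DialogueLoop call locks player movement and shows the next row with its sound.
; After the last row it restores walking, then destroys touch-activated talkers or rewinds others and calls DialogueFinished.
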(event OnComponentBeginOverlap(CollisionComponent)
  (params (OverlappedComponent :type Primitive%20Component%20Object%20Reference) (OtherActor :type Actor%20Object%20Reference) (OtherComp :type Primitive%20Component%20Object%20Reference) (OtherBodyIndex :type Integer) (bFromSweep :type Boolean) (SweepResult :type Hit%20Result%20Structure%20%28by%20ref%29))
  (bind _asbp_third_person_character (Utilities|Casting|CastToBP_ThirdPersonCharacter OtherActor))
  (Variables|Default|SetAs%20BP%20Third%20Person%20Character _asbp_third_person_character)
  (bind _asdefault_topdown_hud (Utilities|Casting|CastToDefaultTopdownHUD (HUD|GetHUD (Game|GetPlayerController 0))))
  (Variables|Default|SetWidget%20reference (Variables|/Game/UI/HUD/DefaultTopdownHUD.DefaultTopdownHUD_C|GetDialogue%20Textbox%20reference _asdefault_topdown_hud))
  (if (Variables|Default|GetTouch%20Activated?)
    (Utilities|FlowControl|DoOnce false
      (:Completed
        (CallFunction|DialogueLoop)))))

(event OnComponentEndOverlap(CollisionComponent)
  (params (OverlappedComponent :type Primitive%20Component%20Object%20Reference) (OtherActor :type Actor%20Object%20Reference) (OtherComp :type Primitive%20Component%20Object%20Reference) (OtherBodyIndex :type Integer))
  (Widget|SetVisibility (Variables|Default|GetWidget%20reference) "Hidden"))

(event Custom|ResetDialogue
  (bind _dialogue_table_file (Variables|Default|GetDialogue%20table%20file))
  (Utilities|FlowControl|DoOnce false) ; enters at Reset
)

(event Custom|Remote%20Trigger%20Event
  (bind _asdefault_topdown_hud (Utilities|Casting|CastToDefaultTopdownHUD (HUD|GetHUD (Game|GetPlayerController 0))))
  (Variables|Default|SetWidget%20reference (Variables|/Game/UI/HUD/DefaultTopdownHUD.DefaultTopdownHUD_C|GetDialogue%20Textbox%20reference _asdefault_topdown_hud))
  (if (Variables|Default|GetTouch%20Activated?)
    (Utilities|FlowControl|DoOnce false
      (:Completed
        (CallFunction|DialogueLoop)))))

(event Custom|Dialogue%20Loop
  (bind _dialogue_table_file (Variables|Default|GetDialogue%20table%20file))
  (Pawn|Components|CharacterMovement|DisableMovement (Variables|/Script/Engine.Character|GetCharacterMovement (Variables|Default|GetAs%20BP%20Third%20Person%20Character)))
  (Widget|SetVisibility (Variables|Default|GetWidget%20reference) "Visible")
  (Utilities|FlowControl|DoOnce false
    (:Completed
      ;[1 1 1] Calculate which row to pull
      (bind _outrownames (DataTable|GetDataTableRowNames _dialogue_table_file))
      (if (> (Utilities|Array|Length _outrownames) (Variables|Default|GetIndex))
        (CallFunction|ResetDialogue)
        (bind _returnvalue (Utilities|GetDataTableRow _dialogue_table_file (Utilities|Array|Get(acopy) _outrownames (Variables|Default|GetIndex)))
          (:then
            (Audio|PlaySound2D (.Soundcue (Utilities|Struct|BreakDialogueTemplate_Structure _returnvalue)) 1.0 1.0 0.0 0 0)
            (Variables|/Game/UI/HUD/Dialogue_Textbox.Dialogue_Textbox_C|SetCurrent%20Dialogue%20displayed (Variables|Default|GetWidget%20reference) (.SpokenDialogue (Utilities|Struct|BreakDialogueTemplate_Structure _returnvalue))) ; Which dialogue line to show
            (Variables|Default|SetIndex (+ (Variables|Default|GetIndex) 1))))
        (else
          ;[1 1 1] Reset the dialogue box if there are no more rows
          (CallFunction|ResetDialogue)
          (Widget|SetVisibility (Variables|Default|GetWidget%20reference) "Hidden")
          (Pawn|Components|CharacterMovement|SetMovementMode (Variables|/Script/Engine.Character|GetCharacterMovement (Variables|Default|GetAs%20BP%20Third%20Person%20Character)) "MOVE_Walking" 0)
          (if (Variables|Default|GetTouch%20Activated?)
            (Actor|DestroyActor)
            (else
              (Variables|Default|SetIndex 0)
              (Default|CallDialogueFinished))))))))

(event Custom|Remote%20Leave%20event
  (Widget|SetVisibility (Variables|Default|GetWidget%20reference) "Hidden"))

(fn ConstructionScript)