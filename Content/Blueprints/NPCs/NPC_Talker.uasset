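; NPC Blueprint that plays data-table dialogue, with text and sound, when the player interacts.
; Collision overlap with the third-person character creates the Dialogue_Textbox widget, and leaving removes it.
; Each InteractionEvent disables player movement, shows the widget and advances one row by index through a DoOnce gate.
; After the last row, it restores walking, resets the index and recreates the widget for replay.
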(event OnComponentBeginOverlap(CollisionComponent)
  (params (OverlappedComponent :type Primitive%20Component%20Object%20Reference) (OtherActor :type Actor%20Object%20Reference) (OtherComp :type Primitive%20Component%20Object%20Reference) (OtherBodyIndex :type Integer) (bFromSweep :type Boolean) (SweepResult :type Hit%20Result%20Structure%20%28by%20ref%29))
  (bind _asbp_third_person_character (Utilities|Casting|CastToBP_ThirdPersonCharacter OtherActor))
  (Variables|Default|SetAs%20BP%20Third%20Person%20Character _asbp_third_person_character)
  ;[0.2435 0.5172 1] Dialogue UI creation
  (bind _returnvalue (UserInterface|CreateWidget "/Game/UI/HUD/Dialogue_Textbox.Dialogue_Textbox_C"))
  (UserInterface|Viewport|AddtoViewport _returnvalue 0)
  (Variables|Default|SetWidget%20reference _returnvalue))

(event OnComponentEndOverlap(CollisionComponent)
  (params (OverlappedComponent :type Primitive%20Component%20Object%20Reference) (OtherActor :type Actor%20Object%20Reference) (OtherComp :type Primitive%20Component%20Object%20Reference) (OtherBodyIndex :type Integer))
  (Widget|RemovefromParent (Variables|Default|GetWidget%20reference)))

(event Custom|ResetDialogue
  (bind _dialogue_table_file (Variables|Default|GetDialogue%20table%20file))
  (Utilities|FlowControl|DoOnce false) ; enters at Reset
)

(event Custom|Reset%20Dialogue%20Box
  ;[0.2435 0.5172 1] Dialogue UI creation
  (bind _returnvalue (UserInterface|CreateWidget "/Game/UI/HUD/Dialogue_Textbox.Dialogue_Textbox_C"))
  (UserInterface|Viewport|AddtoViewport _returnvalue 0)
  (Variables|Default|SetWidget%20reference _returnvalue))

(event EventInteractionEvent
  (bind _dialogue_table_file (Variables|Default|GetDialogue%20table%20file))
  ;[1 1 1] Pre-Loop Events. Happen when player interacts
  (Pawn|Components|CharacterMovement|DisableMovement (Variables|/Script/Engine.Character|GetCharacterMovement (Variables|Default|GetAs%20BP%20Third%20Person%20Character)))
  (Widget|SetVisibility (Variables|Default|GetWidget%20reference) "Visible")
  (Utilities|FlowControl|DoOnce false
    (:Completed
      ;[1 1 1] Calculate which row to pull
      (bind _outrownames (DataTable|GetDataTableRowNames _dialogue_table_file))
      (if (> (Utilities|Array|Length _outrownames) (Variables|Default|GetIndex))
        (CallFunction|ResetDialogue)
        (bind _returnvalue (Utilities|GetDataTableRow _dialogue_table_file (Utilities|Array|Get(acopy) _outrownames (Variables|Default|GetIndex)))
          (:then
            (Audio|PlaySound2D (.Soundcue (Utilities|Struct|BreakDialogueTemplate_Structure _returnvalue)) 1.0 1.0 0.0 0 0)
            (Variables|/Game/UI/HUD/Dialogue_Textbox.Dialogue_Textbox_C|SetCurrent%20Dialogue%20displayed (Variables|Default|GetWidget%20reference) (.SpokenDialogue (Utilities|Struct|BreakDialogueTemplate_Structure _returnvalue))) ; Which dialogue line to show
            (Variables|Default|SetIndex (+ (Variables|Default|GetIndex) 1))))
        (else
          ;[1 1 1] Reset the dialogue box if there are no more rows
          (Widget|RemovefromParent (Variables|Default|GetWidget%20reference))
          (CallFunction|ResetDialogue)
          (Pawn|Components|CharacterMovement|SetMovementMode (Variables|/Script/Engine.Character|GetCharacterMovement (Variables|Default|GetAs%20BP%20Third%20Person%20Character)) "MOVE_Walking" 0)
          (Variables|Default|SetIndex 0)
          (CallFunction|ResetDialogueBox))))))

(fn ConstructionScript)