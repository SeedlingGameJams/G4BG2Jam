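; NPC talker variant, apparently for cinematics, whose dialogue is started by a remote event instead of its own trigger.
; RemotePlayDialogue calls the remote trigger, starts the dialogue loop, then binds a finish handler that fires the remote leave event.
; The interact input also calls the dialogue loop.
; A player-pawn cast to TPC_Luna is left disconnected and never runs.
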(event Custom|Remote%20Play%20Dialogue
  (CallFunction|RemoteTriggerEvent)
  (CallFunction|DialogueLoop)
  (EventDispatchers|AssignDialogueFinished (delegate Custom|Remote%20Dialogue%20finished)))

(event Custom|Remote%20Dialogue%20finished
  (CallFunction|RemoteLeaveEvent))

(event Input|EnhancedActionEvents|EnhancedInputActionIA_Interact
  (params (ActionValue :type Boolean) (ElapsedSeconds :type Float%20%28double-precision%29) (TriggeredSeconds :type Float%20%28double-precision%29) (InputAction :type Input%20Action%20Object%20Reference :default "/Game/ThirdPerson/Input/Actions/IA_Interact.IA_Interact"))
  (:Started
    (CallFunction|DialogueLoop)))

(fn ConstructionScript
  (|CallParentFunction))