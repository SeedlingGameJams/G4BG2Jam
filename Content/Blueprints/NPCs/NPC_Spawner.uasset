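; NPC spawner actor that populates an area with a set number of pawns of a configurable class on BeginPlay.
; Each spawn picks a random navigable point within the sphere radius of the SpawnerBounds component, raised slightly above the navmesh.
; Pawns get a random scale per axis, so they can be non-uniformly stretched.
; Each spawned pawn is registered with the AI manager held by the GM_MainLevel game mode.
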(event EventBeginPlay
  (for _index (range 1 (Variables|Default|GetSpawnAmount))
    (CallFunction|SpawnPawn)))

(fn ConstructionScript)

(fn SpawnPawn
  (bind _returnvalue (Math|Random|RandomFloatinRange 0.5 1.0))
  (bind _spawnerbounds (Variables|Default|GetSpawnerBounds))
  (bind (_origin _boxextent _sphereradius) (Collision|GetComponentBounds _spawnerbounds))
  (bind (_randomlocation _returnvalue_2) (Class|NavigationSystemV1|GetRandomLocationinNavigableRadius _origin _sphereradius 0 0))
  (if _returnvalue_2
    (bind _returnvalue_3 (Game|SpawnActorfromClass (Variables|Default|GetPawn%20Class) (Math|Transform|MakeTransform (+ _randomlocation "0.000000,0.000000,100.000000") "0, 0, 0" (Math|Vector|MakeVector _returnvalue _returnvalue _returnvalue)) "Undefined" 0 0))
    (bind _asgm_main_level (Utilities|Casting|CastToGM_MainLevel (Game|GetGameMode)))
    (Default|AddAi (Default|GetAiManger _asgm_main_level) _returnvalue_3)))