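; AI manager Blueprint that culls registered NPCs by their distance from the player character.
; AddAi stores valid spawned AIs in an array, and BeginPlay precomputes the squared deactivation distance to compare against squared distances.
; Every Tick it loops over the array, enabling actor tick, mesh activation and visibility for AIs inside that range and switching them off for those outside.
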(event Custom|AddAi
  (params (NewItem :type NPC%20Roamer%20BASE%20Object%20Reference%20%28by%20ref%29))
  (Utilities|IsValid NewItem
    (:Is%20Valid
      (Utilities|Array|Add (Variables|Default|GetSpawnedAis) NewItem))))

(event EventBeginPlay
  (Variables|Default|SetSqDeacDistance (Math|Float|Square (Variables|Default|GetDeactivateDistance))))

(event EventTick
  (params (DeltaSeconds :type Float%20%28single-precision%29))
  (for _array_element (Variables|Default|GetSpawnedAis)
    (Actor|Tick|SetActorTickEnabled _array_element (< (Transformation|GetSquaredDistanceTo _array_element (Game|GetPlayerCharacter 0)) (Variables|Default|GetSqDeacDistance)))
    (if (< (Transformation|GetSquaredDistanceTo _array_element (Game|GetPlayerCharacter 0)) (Variables|Default|GetSqDeacDistance))
      (Components|Activation|Activate (Variables|/Script/Engine.Character|GetMesh _array_element) false)
      (Rendering|SetVisibility (Variables|/Script/Engine.Character|GetMesh _array_element) true false)
      (else
        (Components|Activation|Deactivate (Variables|/Script/Engine.Character|GetMesh _array_element))
        (Rendering|SetVisibility (Variables|/Script/Engine.Character|GetMesh _array_element) false false)))))