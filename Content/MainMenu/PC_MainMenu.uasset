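; Player controller for the main menu that owns the root menu widget.
; On BeginPlay it creates a CUI_Menu_Base widget as the menu stack, adds it to the viewport, sets UI-only input and hides the SeedlingsInstance loading screen.
; PushMenu and RemoveMenu events forward activatable widgets to that stack, so the controller acts as the entry point for menu changes.
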(event Custom|PushMenu
  (params (ActivatableWidgetClass :type Common%20Activatable%20Widget%20Class%20Reference))
  (Default|PushMenu (Variables|Default|GetMenuStack) ActivatableWidgetClass))

(event Custom|RemoveMenu
  (params (WidgetToRemove :type Common%20Activatable%20Widget%20Object%20Reference))
  (Default|RemoveMenu (Variables|Default|GetMenuStack) WidgetToRemove))

(event EventBeginPlay
  (bind _returnvalue (UserInterface|CreateWidget "/Game/UI/Menu/CUI_Menu_Base.CUI_Menu_Base_C" self))
  (bind _output_get (Variables|Default|SetMenuStack _returnvalue))
  (UserInterface|Viewport|AddtoViewport _output_get 0)
  (Input|SetInputModeUIOnly self 0 "DoNotLock" false)
  (bind _asseedlings_instance (Utilities|Casting|CastToSeedlingsInstance (Game|GetGameInstance)))
  (Default|HideLoadingScreen _asseedlings_instance))

(fn ConstructionScript)