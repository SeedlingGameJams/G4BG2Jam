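; Spline audio actor that keeps a looping-update ambient sound, apparently for a river, at the point on its spline nearest the player.
; BeginPlay spawns the sound attached to the spline, caches the GM_MainLevel game mode, then starts a repeating short-interval timer, presumably driving MoveAudio.
; MoveAudio snaps the sound to the closest spline point to the player character, lifted slightly, so one emitter covers the whole path.
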(event Custom|MoveAudio
  (bind _returnvalue (Game|GetPlayerCharacter 0))
  (bind _spline (Variables|Default|GetSpline))
  (bind _returnvalue_2 (Transformation|GetActorLocation _returnvalue))
  (bind _returnvalue_3 (Spline|FindLocationClosesttoWorldLocation _spline _returnvalue_2 "World"))
  (Transformation|SetWorldLocation (Variables|Default|GetPlayingSound) (Math|Vector|MakeVector (.x _returnvalue_3) (.y _returnvalue_3) (+ (.z _returnvalue_3) 0.1)) false false))

(event EventBeginPlay
  (bind _returnvalue (Audio|SpawnSoundAttached (Variables|Default|GetSound) (Variables|Default|GetSpline) "None" "0, 0, 0" "0, 0, 0" "KeepRelativeOffset" false 1.0 1.0 0.0 0 0))
  (Variables|Default|SetPlayingSound _returnvalue)
  (bind _asgm_main_level (Utilities|Casting|CastToGM_MainLevel (Game|GetGameMode)))
  (Variables|Default|SetAs%20GM%20Main%20Level _asgm_main_level)
  (if (not (Class|KismetSystemLibrary|TimerExistsHandle (Variables|Default|GetTmrUpdateTime)))
    (bind _returnvalue_2 (Utilities|Time|SetTimerbyEvent (EventDispatchers|CreateEvent :!event Custom|MoveAudio) 0.1 true))
    (Variables|Default|SetTmrUpdateTime _returnvalue_2)))

(fn ConstructionScript)