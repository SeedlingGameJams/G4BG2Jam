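; Creek ambience actor that keeps an audio source at the spline point nearest the third-person player, slightly raised above the river.
; On BeginPlay it starts a fast looping timer, presumably driving the MoveAudio repositioning, and subscribes to every water zone's update event.
; When a zone reports a water type, the enum name is fired as a trigger parameter on the audio source to change the sound.
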(event Custom|MoveAudio
  (bind _as_bp_third_person_character (Variables|Default|GetAs%20BP%20Third%20Person%20Character))
  (bind _spline (Variables|Default|GetSpline))
  (bind _returnvalue (Transformation|GetActorLocation _as_bp_third_person_character))
  (bind _returnvalue_2 (Spline|FindLocationClosesttoWorldLocation _spline _returnvalue "World"))
  (Transformation|SetWorldLocation (Variables|Default|GetAudioSource) (Math|Vector|MakeVector (.x _returnvalue_2) (.y _returnvalue_2) (+ (.z _returnvalue_2) 0.1)) false false))

(event Custom|UpdateWaterType_Event
  (params (CurrentWaterZone :type EWaterZone%20Enum :default "NewEnumerator0"))
  (CallFunction|UpdateWaterType CurrentWaterZone))

(event EventBeginPlay
  (bind _asbp_third_person_character (Utilities|Casting|CastToBP_ThirdPersonCharacter (Game|GetPlayerCharacter 0)))
  (Variables|Default|SetAs%20BP%20Third%20Person%20Character _asbp_third_person_character)
  (bind _outactors (Actor|GetAllActorsOfClass "/Game/Audio/AudioBPs/BP_AxWaterZones.BP_AxWaterZones_C"))
  (for _array_element _outactors
    (EventDispatchers|AssignUpdateWaterType _array_element (delegate Custom|UpdateWaterType_Event)))
  (if (not (Class|KismetSystemLibrary|TimerExistsHandle (Variables|Default|GetTmrUpdateTime)))
    (bind _returnvalue (Utilities|Time|SetTimerbyEvent (EventDispatchers|CreateEvent :!event Custom|MoveAudio) 0.1 true))
    (Variables|Default|SetTmrUpdateTime _returnvalue)))

(fn ConstructionScript)

(fn UpdateWaterType
  (params (WaterType :type EWaterZone%20Enum :default "NewEnumerator0"))
  (Class|AudioParameterControllerInterface|SetTriggerParameter (Variables|Default|GetAudioSource) (Utilities|String|StringToName (Utilities|String|EnumtoString WaterType))))