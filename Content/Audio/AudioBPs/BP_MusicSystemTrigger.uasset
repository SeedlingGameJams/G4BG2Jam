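; BP_MusicSystemTrigger is a music trigger actor that starts and stops a chosen piece of music as the player moves in and out of it.
; Its begin and end overlap events react only to the player 0 character.
; They call PlayMusic on entry and StopMusic on exit, passing MusicToTrigger, and leave the playback itself to logic outside this graph.
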(event Collision|EventActorBeginOverlap
  (params (OtherActor :type Actor%20Object%20Reference))
  (if (== OtherActor (Game|GetPlayerCharacter 0))
    (Default|CallPlayMusic (Variables|Default|GetMusicToTrigger))))

(event Collision|EventActorEndOverlap
  (params (OtherActor :type Actor%20Object%20Reference))
  (if (== OtherActor (Game|GetPlayerCharacter 0))
    (Default|CallStopMusic (Variables|Default|GetMusicToTrigger))))

(fn ConstructionScript)