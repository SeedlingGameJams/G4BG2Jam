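; Audio trigger volume meant to change river loudness in the ambience control bus mix when BP_AxWaterSpline enters or leaves its Box.
; On begin and end overlap it loads CBM_Ambience stages from profile, builds a River stage offset down or up by LoudnessDb, then calls UpdateMix.
; The ArraySet nodes that would insert the adjusted stage are disconnected, so UpdateMix receives the loaded stages unchanged.
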(event OnComponentBeginOverlap(Box)
  (params (OverlappedComponent :type Primitive%20Component%20Object%20Reference) (OtherActor :type Actor%20Object%20Reference) (OtherComp :type Primitive%20Component%20Object%20Reference) (OtherBodyIndex :type Integer) (bFromSweep :type Boolean) (SweepResult :type Hit%20Result%20Structure%20%28by%20ref%29))
  (if (== OtherActor "/Game/Audio/AudioBPs/BP_AxWaterSpline.BP_AxWaterSpline")
    (bind _returnvalue (Class|AudioModulationStatics|LoadMixfromProfile "/Game/Audio/Mixing/CBM_Ambience.CBM_Ambience"))
    (Variables|Default|SetStages _returnvalue)
    (bind _returnvalue_2 (Class|AudioModulationStatics|CreateBusMixStage (.Bus (Utilities|Struct|BreakSoundControlBusMixStage (Utilities|Array|Get(acopy) _returnvalue (Utilities|Array|FindItem _returnvalue (Variables|Default|GetRiver))))) (- (.TargetValue (Utilities|Struct|BreakSoundModulationMixValue (.Value (Utilities|Struct|BreakSoundControlBusMixStage (Utilities|Array|Get(acopy) _returnvalue (Utilities|Array|FindItem _returnvalue (Variables|Default|GetRiver))))))) (Variables|Default|GetLoudnessDb))))
    (Class|AudioModulationStatics|UpdateMix "/Game/Audio/Mixing/CBM_Ambience.CBM_Ambience" (Variables|Default|GetStages) -1.0)))

(event OnComponentEndOverlap(Box)
  (params (OverlappedComponent :type Primitive%20Component%20Object%20Reference) (OtherActor :type Actor%20Object%20Reference) (OtherComp :type Primitive%20Component%20Object%20Reference) (OtherBodyIndex :type Integer))
  (if (== OtherActor "/Game/Audio/AudioBPs/BP_AxWaterSpline.BP_AxWaterSpline")
    (bind _returnvalue (Class|AudioModulationStatics|LoadMixfromProfile "/Game/Audio/Mixing/CBM_Ambience.CBM_Ambience"))
    (Variables|Default|SetStages _returnvalue)
    (bind _returnvalue_2 (Class|AudioModulationStatics|CreateBusMixStage (.Bus (Utilities|Struct|BreakSoundControlBusMixStage (Utilities|Array|Get(acopy) _returnvalue (Utilities|Array|FindItem _returnvalue (Variables|Default|GetRiver))))) (+ (.TargetValue (Utilities|Struct|BreakSoundModulationMixValue (.Value (Utilities|Struct|BreakSoundControlBusMixStage (Utilities|Array|Get(acopy) _returnvalue (Utilities|Array|FindItem _returnvalue (Variables|Default|GetRiver))))))) (Variables|Default|GetLoudnessDb))))
    (Class|AudioModulationStatics|UpdateMix "/Game/Audio/Mixing/CBM_Ambience.CBM_Ambience" (Variables|Default|GetStages) -1.0)))

(fn ConstructionScript)