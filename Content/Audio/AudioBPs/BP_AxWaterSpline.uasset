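; Water ambience actor that keeps a single audio source at the point on a river spline nearest the player.
; A looping timer, rather than Tick, refreshes the source position, lifting it slightly above the river.
; On BeginPlay it subscribes to every BP_AxWaterZones actor's water-type update, converting the reported enum to a name that fires the matching trigger parameter on the audio source.
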(event Custom|MoveAudio
  (bind _returnvalue (Game|GetPlayerCharacter 0))
  (bind _spline (Variables|Default|GetSpline))
  (bind _returnvalue_2 (Transformation|GetActorLocation _returnvalue))
  (bind _returnvalue_3 (Spline|FindLocationClosesttoWorldLocation _spline _returnvalue_2 "World"))
  (Transformation|SetWorldLocation (Variables|Default|GetAudioSource) (Math|Vector|MakeVector (.x _returnvalue_3) (.y _returnvalue_3) (+ (.z _returnvalue_3) 0.1)) false false))

(event Custom|UpdateWaterType_Event
  (params (CurrentWaterZone :type EWaterZone%20Enum :default "NewEnumerator0"))
  (CallFunction|UpdateWaterType CurrentWaterZone))

(event EventBeginPlay
  (bind _outactors (Actor|GetAllActorsOfClass "/Game/Audio/AudioBPs/BP_AxWaterZones.BP_AxWaterZones_C"))
  (for _array_element _outactors
    (EventDispatchers|AssignUpdateWaterType _array_element (delegate Custom|UpdateWaterType_Event)))
  (if (not (Class|KismetSystemLibrary|TimerExistsHandle (Variables|Default|GetTmrUpdateTime)))
    (bind _returnvalue (Utilities|Time|SetTimerbyEvent (EventDispatchers|CreateEvent :!event Custom|MoveAudio) 0.1 true))
    (Variables|Default|SetTmrUpdateTime _returnvalue)))

(fn ConstructionScript)

(fn UpdateWaterType
  (params (WaterType :type EWaterZone%20Enum :default "NewEnumerator0"))
  (Class|AudioParameterControllerInterface|SetTriggerParameter (Variables|Default|GetAudioSource) (Utilities|String|StringToName (Utilities|String|EnumtoString WaterType))))