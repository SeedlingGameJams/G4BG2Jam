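; BP_MusicSystem is the level's music manager, driving one audio component through named trigger parameters.
; One tick after BeginPlay, the tutorial level instead loads a Soundscape palette collection and sets the Storm state.
; Other levels start the audio on the Calm3 track and bind to every BP_MusicSystemTrigger's play and stop events.
; Those handlers build trigger names by prefixing the music enum's name with "Play" or "Stop".
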(event Custom|PlayMusic_Event
  (params (MusicToPlay :type EMusicTypes%20Enum :default "NewEnumerator0"))
  (Class|AudioParameterControllerInterface|SetTriggerParameter (Variables|Default|GetAudio) (Utilities|String|StringToName (Utilities|String|Append "Play" (Utilities|String|EnumtoString MusicToPlay)))))

(event Custom|StopMusic_Event
  (params (MusicToStop :type EMusicTypes%20Enum :default "NewEnumerator0"))
  (Class|AudioParameterControllerInterface|SetTriggerParameter (Variables|Default|GetAudio) (Utilities|String|StringToName (Utilities|String|Append "Stop" (Utilities|String|EnumtoString MusicToStop)))))

(event EventBeginPlay
  (bind _returnvalue (Subsystems|GetSoundscapeSubsystem))
  (Utilities|FlowControl|DelayUntilNextTick)
  ;[1 1 1] Are we in the tutorial level?
  (if (== (Class|Actor|GetLevel) 0)
    (Class|SoundscapeSubsystem|AddPaletteCollection _returnvalue "Tutoeial" (Variables|Default|GetPalette%20Collection))
    (Class|SoundscapeSubsystem|SetState _returnvalue "(TagName=\"Soundscape.Storm\")")
    (else
      (Audio|Components|Audio|Play (Variables|Default|GetAudio) 0.0)
      (Class|AudioParameterControllerInterface|SetTriggerParameter (Variables|Default|GetAudio) "PlayCalm3")
      (bind _outactors (Actor|GetAllActorsOfClass "/Game/Audio/AudioBPs/BP_MusicSystemTrigger.BP_MusicSystemTrigger_C"))
      (for _array_element _outactors
        (EventDispatchers|AssignPlayMusic _array_element (delegate Custom|PlayMusic_Event))
        (EventDispatchers|AssignStopMusic _array_element (delegate Custom|StopMusic_Event))))))

(fn ConstructionScript)