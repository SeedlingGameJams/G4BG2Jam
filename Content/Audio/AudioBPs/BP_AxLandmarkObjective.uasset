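; Landmark objective actor that reacts to echo pings with a positional sound and an outline highlight.
; On BeginPlay it picks its sound from the SoundKey map using its DebugTitle enum.
; An echo hit plays that sound attached to the root and turns on the mesh's custom depth; echo end turns it off.
; The construction script shows the enum name on a text render component for identification.
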(event EventEchoEnd
  (Rendering|SetRenderCustomDepth (Variables|Default|GetLandmarkMesh) false))

(event EventEchoHit
  (Audio|SpawnSoundAttached (Variables|Default|GetFileToPlay) (Variables|Default|GetDefaultSceneRoot) "None" "0, 0, 0" "0, 0, 0" "KeepRelativeOffset" false 1.0 1.0 0.0 0 0)
  (Rendering|SetRenderCustomDepth (Variables|Default|GetLandmarkMesh) true))

(event EventBeginPlay
  (Variables|Default|SetFileToPlay (.Value (Utilities|Map|Find (Variables|Default|GetSoundKey) (Variables|Default|GetDebugTitle)))))

(fn ConstructionScript
  (Rendering|Components|TextRender|SetText (Variables|Default|GetTextRender) (Utilities|Text|ToText(String) (Utilities|String|EnumtoString (Variables|Default|GetDebugTitle)))))