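; Audio spline actor that keeps a looping-style attached sound positioned along a spline relative to the player.
; On BeginPlay it spawns the configured sound attached to the spline, and deactivates it when the actor is destroyed.
; Each tick it moves the sound to the spline point closest to player 0.
; With PlaySoundAhead set, it instead offsets that point a fixed distance along the spline's direction there.
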(event Custom|OnDestroyed_Event
  (params (DestroyedActor :type Actor%20Object%20Reference))
  (Components|Activation|Deactivate (Variables|Default|GetPlayingSound)))

(event EventBeginPlay
  (bind _returnvalue (Audio|SpawnSoundAttached (Variables|Default|GetSound) (Variables|Default|GetSpline) "None" "0, 0, 0" "0, 0, 0" "KeepRelativeOffset" false 1.0 1.0 0.0 0 0))
  (Variables|Default|SetPlayingSound _returnvalue)
  (Game|AssignOnDestroyed (delegate Custom|OnDestroyed_Event)))

(event EventTick
  (params (DeltaSeconds :type Float%20%28single-precision%29))
  (bind _returnvalue (Game|GetPlayerCharacter 0))
  (bind _spline (Variables|Default|GetSpline))
  (bind _returnvalue_2 (Transformation|GetActorLocation _returnvalue))
  (bind _returnvalue_3 (Spline|FindLocationClosesttoWorldLocation _spline _returnvalue_2 "World"))
  (Utilities|IsValid _returnvalue
    (:Is%20Valid
      (if (Variables|Default|GetPlaySoundAhead)
        (Transformation|SetWorldLocation (Variables|Default|GetPlayingSound) (+ (* (Spline|FindDirectionClosesttoWorldLocation _spline _returnvalue_2 "World") 1.5e+03) _returnvalue_3) false false)
        (else
          (Transformation|SetWorldLocation (Variables|Default|GetPlayingSound) (+ _returnvalue_3 "0.000000,0.000000,1.000000") false false))))))

(fn ConstructionScript)